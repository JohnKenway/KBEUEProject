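; LoginGameMode is the game mode for the login screen, linking the login widget to KBEngine-style events.
; On BeginPlay it creates LoginWidget, adds it to the viewport and binds the widget's Say delegate to forward messages to Say.
; OnSay casts its event data to KBEventData_OnSay and prints the message on screen.
; OnLoginSuccessed prints a success message and notifies the widget.
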(event Custom|自定义事件_0
  (params (Msg :type String))
  (Class|LoginModeBase|Say Msg))

(event EventBeginPlay
  (bind _returnvalue (UserInterface|CreateWidget "/Game/Blueprint/LoginWidget.LoginWidget_C"))
  (UserInterface|Viewport|AddtoViewport _returnvalue 0)
  (bind _output_get (Variables|Default|SetLoginWidget _returnvalue))
  (EventDispatchers|BindEventtoSayDele _output_get (delegate Custom|自定义事件_0)))

(event EventTick
  (params (DeltaSeconds :type Float%20%28single-precision%29)))

(event EventOnSay
  (params (EventData :type KB%20Event%20Data%20Object%20Reference))
  (bind _askbevent_data_on_say (Utilities|Casting|CastToKBEventData_OnSay EventData))
  (Development|PrintString (Variables|/Script/KBEnginePlugins.KBEventData_OnSay|GetMsg _askbevent_data_on_say) true true "(R=0.000000,G=0.660000,B=1.000000,A=1.000000)" 2e+01))

(event EventOnLoginSuccessed
  (params (EventData :type KB%20Event%20Data%20Object%20Reference))
  (Development|PrintString "Login Success" true true "(R=0.000000,G=0.660000,B=1.000000,A=1.000000)" 5e+03)
  (Default|LoginSuccessed (Variables|Default|GetLoginWidget)))

(fn ConstructionScript)